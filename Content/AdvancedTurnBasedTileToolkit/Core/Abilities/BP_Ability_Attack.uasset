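; Attack ability for the turn-based tile toolkit, in which the owning unit damages a target unit on the grid.
; Damage is copied from the owning unit when unit attributes are in use.
; Execution looks up the unit at the target index and queues the attack on the owner with a post-hit delay.
; Target value is inverse current health capped at one, so weaker units score higher.
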(event EventUpdateAttributes
  (|CallParentFunction)
  (if (Variables|Default|GetbUseUnitAttributes)
    (Variables|Default|SetDamage (Variables|/Game/AdvancedTurnBasedTileToolkit/Core/Units/BP_Unit.BP_Unit_C|GetDamage (Variables|Default|GetOwningUnit)))))

(fn ConstructionScript
  (|CallParentFunction))

(fn FindTargetValue
  (params (TargetIndex :type Integer))
  (return (Math|Float|Min(Float) (/ 1.0 (Variables|/Game/AdvancedTurnBasedTileToolkit/Core/Units/BP_Unit.BP_Unit_C|GetCurrentHealth (.Value (Utilities|Map|Find (Variables|/Game/AdvancedTurnBasedTileToolkit/Core/Grid/BP_GridManager.BP_GridManager_C|GetGridUnits (Variables|Default|GetGridManagerRef)) TargetIndex)))) 1.0)))

(fn GetDescription
  (return "Attack" "Attack a target in range."))

(fn ExecuteAbility
  (params (TargetIndexIn :type Integer))
  (Default|QueueAttackUnit (Variables|Default|GetOwningUnit) (.Value (Utilities|Map|Find (Variables|/Game/AdvancedTurnBasedTileToolkit/Core/Grid/BP_GridManager.BP_GridManager_C|GetGridUnits (Variables|Default|GetGridManagerRef)) TargetIndexIn)) (Variables|Default|GetDamage) (Variables|Default|GetPostHitDelay))
  (return true))