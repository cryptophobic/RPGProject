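; BP_Actor_Puppet_Big is the puppet actor for multi-tile big units in the turn-based tile toolkit.
; On setup from its unit, it runs the parent setup, then reads the paired BP_Unit_Big's Size.
; Even sizes store an offset of half the grid manager's tile X size on both X and Y, which GetPuppetOffset returns.
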(event EventSetupfromUnit
  (params (Unit :type Actor%20Object%20Reference))
  (bind _gridmanager (CallFunction|GetGridManager))
  (bind _tilexsize (Variables|/Game/AdvancedTurnBasedTileToolkit/Core/Grid/BP_GridManager.BP_GridManager_C|GetTileXSize _gridmanager))
  (bind _returnvalue (/ _tilexsize 2.0))
  (|CallParentFunction Unit)
  (bind _asbp_unit_big (Utilities|Casting|CastToBP_Unit_Big (Variables|Default|GetPairedUnit)))
  (if (Utilities|IsEven (Variables|/Game/AdvancedTurnBasedTileToolkit/Maps/Experimental/BigUnits/BP_Unit_Big.BP_Unit_Big_C|GetSize _asbp_unit_big))
    (Variables|Default|SetOffset (Math|Vector|MakeVector _returnvalue _returnvalue 0.0))))

(fn ConstructionScript
  (|CallParentFunction))

(fn GetPuppetOffset
  (return (Variables|Default|GetOffset)))